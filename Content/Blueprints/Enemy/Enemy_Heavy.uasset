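; Heavy enemy Blueprint that chases the player and deals damage on reaching them.
; BeginPlay randomizes mesh scale, yaw and walk speed, then starts a self-repeating AIMoveTo loop that applies damage after a short delay on success and retries on failure.
; AnyDamage reduces clamped health; at zero, a timeline update moves it toward a random point ahead of the player, fires Onkilled, destroys it and spawns a particle effect.
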(event Custom|Chase%20Player
  (params (Player%20to%20chase :type Cube%20Player%20Character%20Object%20Reference))
  ;[1 1 1] AI Chase Player
  (AI|AIMoveTo self "0, 0, 0" Player%20to%20chase 5.0 false
    (:OnSuccess
      (Utilities|FlowControl|Delay 0.25)
      (Game|Damage|ApplyDamage (Game|GetPlayerCharacter 0) (Variables|Default|GetHeavy%20Damage) 0 0)
      (Development|PrintString "Player Damaged" true true "(R=1.000000,G=0.956041,B=0.000000,A=1.000000)"))
    (:OnFail
      _))
  (CallFunction|ChasePlayer (Variables|Default|GetCharacter%20Reference)))

(event EventBeginPlay
  (bind _returnvalue (Math|Random|RandomFloatinRange 0.9 1.1))
  ;[1 1 1] AI Chase Player
  (Transformation|SetWorldScale3D (Variables|Character|GetMesh) (Math|Vector|MakeVector _returnvalue _returnvalue _returnvalue))
  (Transformation|SetActorRotation (Math|Rotator|MakeRotator 0.0 0.0 (Math|Random|RandomFloatinRange 0.0 3.6e+02)))
  (Variables|/Script/Engine.CharacterMovementComponent|SetMaxWalkSpeed (Variables|Character|GetCharacterMovement) (Math|Random|RandomFloatinRange 3e+02 6e+02))
  (bind _ascube_player_character (Utilities|Casting|CastToCube_PlayerCharacter (Game|GetPlayerCharacter 0)))
  (bind _output_get (Variables|Default|SetCharacter%20Reference _ascube_player_character))
  (CallFunction|ChasePlayer _output_get))

(event Game|Damage|EventAnyDamage
  (params (Damage :type Float%20%28single-precision%29) (DamageType :type Damage%20Type%20Object%20Reference) (InstigatedBy :type Controller%20Object%20Reference) (DamageCauser :type Actor%20Object%20Reference))
  (bind _returnvalue (Game|GetPlayerCharacter 0))
  ;[1 1 1] Take Damage / Death
  (bind _output_get (Variables|Default|SetHeavy%20Health (Math|Float|Clamp(Float) (- (Variables|Default|GetHeavy%20Health) Damage) 0.0 3e+02)))
  (if (== _output_get 0.0)
    (bind _output_get_2 (Variables|Default|SetPushBackLocation (+ (* (Transformation|GetActorForwardVector _returnvalue) (Math|Random|RandomFloatinRange 5e+02 1e+03)) (Transformation|GetActorLocation _returnvalue))))
    (bind _newtrack_0 (Timeline|Timeline_0 PlayFromStart)
      (:Update
        (Transformation|SetActorLocation (Math|Vector|MakeVector (Math|Float|Lerp (.X (Math|Vector|BreakVector (Transformation|GetActorLocation))) (.x _output_get_2) _newtrack_0) (.y _output_get_2) (.z _output_get_2)) false false)
        (Default|CallOnkilled self)
        (Actor|DestroyActor)
        (Effects|SpawnEmitteratLocation "/Engine/Tutorial/SubEditors/TutorialAssets/TutorialParticleSystem.TutorialParticleSystem" (Transformation|GetActorLocation))))))

(fn ConstructionScript)
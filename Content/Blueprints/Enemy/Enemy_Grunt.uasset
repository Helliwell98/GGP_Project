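; Melee grunt enemy that chases the player and, on reaching them, plays a flashing sequencer attack that damages them if inside DamBox.
; Damage briefly turns on capsule physics as a ragdoll stagger before the chase resumes.
; Death releases the beanie and knife, reveals hidden cubes and fires OnKilled, with separate events for health drop and destruction.
; Failed moves start a velocity-based stuck check whose MultiGate counts retries before killing the grunt.
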(event Custom|GruntDeath
  ;[1 1 1] Take Damage / Death
  (Physics|SetSimulatePhysics (Variables|Default|GetSuper_Cool_Beanie) true)
  (Development|SetHiddeninGame (Variables|Default|GetCube2) false false)
  (Default|CallOnkilled self))

(event Custom|DropHealthPickup
  (bind _returnvalue (Transformation|GetActorLocation))
  (bind _outhit (Collision|LineTraceByChannel _returnvalue (+ _returnvalue (* (* (Math|Vector|GetUpVector (Transformation|GetActorRotation)) -1) 500)) "TraceTypeQuery1" false 0 "Persistent"))
  (Game|SpawnActorfromClass "/Game/James/HealthPlusOne.HealthPlusOne_C" (Math|Transform|MakeTransform (Math|Vector|MakeVector (.x (.location _outhit)) (.y (.location _outhit)) (+ (.z (.location _outhit)) 25.0)) "0, 0, 0" "1,1,1") "AdjustIfPossibleButAlwaysSpawn" 0 0))

(event Custom|DestroyMe
  ;[1 1 1] Take Damage / Death
  (Utilities|FlowControl|Delay 2.0)
  (Actor|DestroyActor))

(event Custom|Chase%20Player
  (params (Player%20to%20chase :type Cube%20Player%20Character%20Object%20Reference))
  (bind _character_reference (Variables|Default|GetCharacter%20Reference))
  ;[1 1 1] AI Chase Player
  (if (not (Variables|Default|GetisRagdolling))
    (AI|AIMoveTo self "0, 0, 0" Player%20to%20chase 2e+02 false
      (:OnSuccess
        (Components|Movement|StopMovementImmediately (Variables|Character|GetCharacterMovement))
        (Rendering|Material|CreateDynamicMaterialInstance (Variables|Default|GetSphere) 0 "/Game/Jay/M_AttackFlash.M_AttackFlash" "None" :!class /Script/Engine.PrimitiveComponent)
        (Sequencer|Player|Play (Variables|/Script/ActorSequence.ActorSequenceComponent|GetSequencePlayer (Variables|Default|GetAttack)) :!class /Script/MovieScene.MovieSceneSequencePlayer)
        (Utilities|FlowControl|Delay (/ 1.5 (Components|Animation|GetPlayRate (Variables|/Script/ActorSequence.ActorSequenceComponent|GetSequencePlayer (Variables|Default|GetAttack)))))
        (Rendering|Material|CreateDynamicMaterialInstance (Variables|Default|GetSphere) 0 "/Game/Blueprints/Player/CubeMattEnemy.CubeMattEnemy" "None" :!class /Script/Engine.PrimitiveComponent)
        (if (Collision|IsOverlappingActor (Variables|Default|GetDamBox) _character_reference :!class /Script/Engine.PrimitiveComponent)
          (if (not (Variables|Default|GetisRagdolling))
            (Game|Damage|ApplyDamage _character_reference (Variables|Default|GetGrunt%20Damage) 0 0)
            (Utilities|FlowControl|Delay 0.3 :!label _label)
            (CallFunction|ChasePlayer (Variables|Default|GetCharacter%20Reference) :!label _label_2))
          (else
            (goto _label))))
      (:OnFail
        (CallFunction|MovementTest)
        (goto _label_2)))))

(event Custom|MovementTest
  (if (Math|Vector|Equal(Vector) (Variables|/Script/Engine.MovementComponent|GetVelocity (Variables|Character|GetCharacterMovement)) "0, 0, 0" 0.0001)
    (bind _returnvalue (Utilities|Time|SetTimerbyEvent (delegate Custom|Test) 1.0 true))
    (else
      (Development|PrintString "NOT STUCK"))))

(event Custom|Test
  (Utilities|FlowControl|Delay 1.0)
  (if (Math|Vector|Equal(Vector) (Variables|/Script/Engine.MovementComponent|GetVelocity (Variables|Character|GetCharacterMovement)) "0, 0, 0" 0.0001)
    (Utilities|FlowControl|MultiGate false false -1 :!label _label
      (:Out%200
        (CallFunction|Test :!label _label_2)
        (Development|PrintString "TESTING"))
      (:Out%201
        (goto _label_2))
      (:Out%202
        (goto _label_2))
      (:Out%203
        (goto _label_2))
      (:Out%204
        (goto _label_2))
      (:Out%205
        (CallFunction|GruntDeath)))
    (else
      (Utilities|FlowControl|Sequence
        (:then_0
          (goto _label Reset))
        (:then_1
          (Utilities|Time|ClearandInvalidateTimerbyHandle (stale Custom|MovementTest _returnvalue)))))))

(event EventBeginPlay
  (bind _returnvalue (Math|Random|RandomFloatinRange 0.9 1.1))
  ;[1 1 1] AI Chase Player
  (Development|SetHiddeninGame (Variables|Default|GetCube2) true false)
  (Transformation|SetWorldScale3D (Variables|Character|GetMesh) (Math|Vector|MakeVector _returnvalue _returnvalue _returnvalue))
  (Transformation|SetActorRotation (Math|Rotator|MakeRotator 0.0 0.0 (Math|Random|RandomFloatinRange 0.0 3.6e+02)))
  (bind _ascube_player_character (Utilities|Casting|CastToCube_PlayerCharacter (Game|GetPlayerCharacter 0)))
  (bind _output_get (Variables|Default|SetCharacter%20Reference _ascube_player_character))
  (CallFunction|ChasePlayer _output_get))

(event Game|Damage|EventAnyDamage
  (params (Damage :type Float%20%28single-precision%29) (DamageType :type Damage%20Type%20Object%20Reference) (InstigatedBy :type Controller%20Object%20Reference) (DamageCauser :type Actor%20Object%20Reference))
  (bind _capsulecomponent (Variables|Collision|GetCapsuleComponent))
  ;[1 1 1] Take Damage / Death
  (if (not (Variables|Default|GetisRagdolling))
    (bind _output_get (Variables|Default|SetGruntHealth (- (Variables|Default|GetGruntHealth) Damage)))
    (if (<= _output_get 0.0)
      (CallFunction|GruntDeath))
    ;;[1 1 1] Ragdoll (Remove chase player)
    (Audio|PlaySound2D "/Game/Audio/Enemy_Damaged1_Cue.Enemy_Damaged1_Cue" 1.0 1.0 0.0 0 0)
    (Variables|Default|SetisRagdolling true)
    (Class|MovieSceneSequencePlayer|StopatCurrentTime (Variables|/Script/ActorSequence.ActorSequenceComponent|GetSequencePlayer (Variables|Default|GetAttack)))
    (Components|Movement|StopMovementImmediately (Variables|Character|GetCharacterMovement))
    (Physics|SetSimulatePhysics _capsulecomponent true)
    (Utilities|FlowControl|Delay 2.0)
    (Physics|SetSimulatePhysics _capsulecomponent false)
    (Variables|Default|SetisRagdolling false)
    (Transformation|SetWorldRotation (Variables|Collision|GetCapsuleComponent) "0, 0, 0" false false)
    (CallFunction|ChasePlayer (Variables|Default|GetCharacter%20Reference))))

(fn ConstructionScript)
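; Door_BP is a two-panel sliding door for the City Street level that the player toggles with F or the gamepad right shoulder.
; Box overlap enables player 0 input and opens a Gate, and end overlap reverses both, without filtering the overlapping actor.
; When DoorOpenActive is true, presses pass the Gate into a FlipFlop that plays or reverses a Timeline lerping Left and Right apart along X.
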(event OnComponentBeginOverlap(Box)
  (params (OverlappedComponent :type Primitive%20Component%20Object%20Reference) (OtherActor :type Actor%20Object%20Reference) (OtherComp :type Primitive%20Component%20Object%20Reference) (OtherBodyIndex :type Integer) (bFromSweep :type Boolean) (SweepResult :type Hit%20Result%20Structure%20%28by%20ref%29))
  (Input|EnableInput (Game|GetPlayerController 0))
  (Utilities|FlowControl|Gate true) ; enters at Open
)

(event OnComponentEndOverlap(Box)
  (params (OverlappedComponent :type Primitive%20Component%20Object%20Reference) (OtherActor :type Actor%20Object%20Reference) (OtherComp :type Primitive%20Component%20Object%20Reference) (OtherBodyIndex :type Integer))
  (Input|DisableInput (Game|GetPlayerController 0))
  (Utilities|FlowControl|Gate true) ; enters at Close
)

(event Input|KeyboardEvents|F
  (params (Key :type Key%20Structure))
  (:Pressed
    (if (Variables|Default|GetDoorOpenActive)
      (Utilities|FlowControl|Gate true
        (:Exit
          (Utilities|FlowControl|FlipFlop
            (:A
              (bind _newtrack_0 (Timeline|Timeline_0 Play)
                (:Update
                  (Transformation|SetRelativeLocation (Variables|Default|Getleft) (Math|Vector|MakeVector (Math|Float|Lerp -87.5 -200.5 _newtrack_0) 0.0 0.0) false false)
                  (Transformation|SetRelativeLocation (Variables|Default|Getright) (Math|Vector|MakeVector (Math|Float|Lerp 87.5 200.5 _newtrack_0) 0.0 0.0) false false))))
            (:B
              (Timeline|Timeline_0 Reverse))))))))

(event Input|GamepadEvents|GamepadRightShoulder
  (params (Key :type Key%20Structure))
  (:Pressed
    (if (Variables|Default|GetDoorOpenActive)
      (Utilities|FlowControl|Gate true
        (:Exit
          (Utilities|FlowControl|FlipFlop
            (:A
              (bind _newtrack_0 (Timeline|Timeline_0 Play)
                (:Update
                  (Transformation|SetRelativeLocation (Variables|Default|Getleft) (Math|Vector|MakeVector (Math|Float|Lerp -87.5 -200.5 _newtrack_0) 0.0 0.0) false false)
                  (Transformation|SetRelativeLocation (Variables|Default|Getright) (Math|Vector|MakeVector (Math|Float|Lerp 87.5 200.5 _newtrack_0) 0.0 0.0) false false))))
            (:B
              (Timeline|Timeline_0 Reverse))))))))

(fn ConstructionScript)
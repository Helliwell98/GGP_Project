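; Director actor that manages the population of Enemy_Heavy creatures and fulfills horde spawner requests.
; On BeginPlay it registers every existing heavy enemy and Hordespawner_2, binding to their killed and spawn-request events.
; Spawn requests create enemies at random reachable points near the requested location, clamped so the tracked count stays within Maxcreatures.
; Killed creatures are removed from the tracked list, freeing room for later spawns.
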(event EventBeginPlay
  (Utilities|FlowControl|Sequence
    (:then_0
      (bind _outactors (Actor|GetAllActorsOfClass "/Game/Blueprints/Enemy/Enemy_Heavy.Enemy_Heavy_C"))
      (for _array_element _outactors
        (CallFunction|Oncreaturespawned _array_element)))
    (:then_1
      (bind _outactors_2 (Actor|GetAllActorsOfClass "/Game/spawn2/zombies/creature/director/hordespawner_2.hordespawner_2_C"))
      (for _array_element_2 _outactors_2
        (CallFunction|Onhordespawnerspawned _array_element_2)))))

(event Collision|EventActorBeginOverlap
  (params (OtherActor :type Actor%20Object%20Reference)))

(event EventTick
  (params (DeltaSeconds :type Float%20%28single-precision%29)))

(fn ConstructionScript)

(fn Oncreaturespawned
  (params (enemyheavy :type Enemy%20Heavy%20Object%20Reference))
  (Utilities|Array|Add (Variables|Default|GetEnemyheavy) enemyheavy)
  (EventDispatchers|BindEventtoOnkilled enemyheavy (EventDispatchers|CreateEvent :!event Oncreaturekilled)))

(fn Oncreaturekilled
  (params (enemyheavy :type Enemy%20Heavy%20Object%20Reference))
  (Utilities|Array|RemoveItem (Variables|Default|GetEnemyheavy) enemyheavy))

(fn Onhordespawnerspawned
  (params (hordespawners :type Hordespawner%202%20Object%20Reference))
  (Utilities|Array|Add (Variables|Default|Gethordespawnerrs) hordespawners)
  (EventDispatchers|BindEventtoRequestspawn hordespawners (EventDispatchers|CreateEvent :!event Oncreaturespawnedrequested)))

(fn Oncreaturespawnedrequested
  (params (count :type Integer) (location :type Vector))
  (for _index (range 1 (Math|Integer|Min(Integer) count (- (Variables|Default|Getmaxcreatures) (Utilities|Array|Length (Variables|Default|GetEnemyheavy)))))
    (bind _returnvalue (Game|SpawnActorfromClass "/Game/Blueprints/Enemy/Enemy_Heavy.Enemy_Heavy_C" (Math|Transform|MakeTransform (+ (.RandomLocation (AI|Navigation|GetRandomReachablePointinRadius location 2e+02 0 0)) "0.000000, 0,100.000000") "0, 0, 0" "1,1,1") "AdjustIfPossibleButDontSpawnIfColliding" 0 0))
    (Utilities|IsValid _returnvalue
      (:Is%20Valid
        (CallFunction|Oncreaturespawned)))))
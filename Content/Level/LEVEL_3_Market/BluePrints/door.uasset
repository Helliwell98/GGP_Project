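; Interactive door for the Market level that swings open and closed when toggled from inside its trigger area.
; Box overlap enables player 0's input and opens a Gate, and end overlap reverses both, without filtering the overlapping actor.
; F or gamepad right shoulder passes the Gate into a FlipFlop that plays or reverses a Timeline, lerping Box1's relative yaw through a quarter turn.
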(event OnComponentBeginOverlap(box)
  (params (OverlappedComponent :type Primitive%20Component%20Object%20Reference) (OtherActor :type Actor%20Object%20Reference) (OtherComp :type Primitive%20Component%20Object%20Reference) (OtherBodyIndex :type Integer) (bFromSweep :type Boolean) (SweepResult :type Hit%20Result%20Structure%20%28by%20ref%29))
  (Input|EnableInput (Game|GetPlayerController 0))
  (Utilities|FlowControl|Gate true) ; enters at Open
)

(event OnComponentEndOverlap(box)
  (params (OverlappedComponent :type Primitive%20Component%20Object%20Reference) (OtherActor :type Actor%20Object%20Reference) (OtherComp :type Primitive%20Component%20Object%20Reference) (OtherBodyIndex :type Integer))
  (Input|DisableInput (Game|GetPlayerController 0))
  (Utilities|FlowControl|Gate true) ; enters at Close
)

(event EventBeginPlay)

(event Collision|EventActorBeginOverlap
  (params (OtherActor :type Actor%20Object%20Reference)))

(event EventTick
  (params (DeltaSeconds :type Float%20%28single-precision%29)))

(event Input|KeyboardEvents|F
  (params (Key :type Key%20Structure :default "None"))
  (:Pressed
    (Utilities|FlowControl|Gate true
      (:Exit
        (Utilities|FlowControl|FlipFlop
          (:A
            (bind _newtrack_0 (Timeline|Timeline_0 Play)
              (:Update
                (Transformation|SetRelativeRotation (Variables|Default|GetBox1) (Math|Rotator|MakeRotator 0.0 0.0 (Math|Float|Lerp 0.0 9e+01 _newtrack_0)) false false))))
          (:B
            (Timeline|Timeline_0 Reverse)))))))

(event Input|GamepadEvents|GamepadRightShoulder
  (params (Key :type Key%20Structure :default "None"))
  (:Pressed
    (Utilities|FlowControl|Gate true
      (:Exit
        (Utilities|FlowControl|FlipFlop
          (:A
            (bind _newtrack_0 (Timeline|Timeline_0 Play)
              (:Update
                (Transformation|SetRelativeRotation (Variables|Default|GetBox1) (Math|Rotator|MakeRotator 0.0 0.0 (Math|Float|Lerp 0.0 9e+01 _newtrack_0)) false false))))
          (:B
            (Timeline|Timeline_0 Reverse)))))))

(fn ConstructionScript)
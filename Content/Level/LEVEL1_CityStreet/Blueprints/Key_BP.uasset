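; Key pickup for the City Street level that unlocks a door when the player presses F nearby.
; Sphere overlap begin and end enable or disable input, toggle the TextRender prompt and open or close a gate on the F key, without filtering the overlapping actor.
; A gated press sets DoorOpenActive on the first Door_BP found in the level, then destroys the key.
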(event OnComponentBeginOverlap(Sphere)
  (params (OverlappedComponent :type Primitive%20Component%20Object%20Reference) (OtherActor :type Actor%20Object%20Reference) (OtherComp :type Primitive%20Component%20Object%20Reference) (OtherBodyIndex :type Integer) (bFromSweep :type Boolean) (SweepResult :type Hit%20Result%20Structure%20%28by%20ref%29))
  (Input|EnableInput (Game|GetPlayerController 0))
  (Rendering|ToggleVisibility (Variables|Default|GetTextRender) false)
  (Utilities|FlowControl|Gate true) ; enters at Open
)

(event OnComponentEndOverlap(Sphere)
  (params (OverlappedComponent :type Primitive%20Component%20Object%20Reference) (OtherActor :type Actor%20Object%20Reference) (OtherComp :type Primitive%20Component%20Object%20Reference) (OtherBodyIndex :type Integer))
  (Input|DisableInput (Game|GetPlayerController 0))
  (Rendering|ToggleVisibility (Variables|Default|GetTextRender) false)
  (Utilities|FlowControl|Gate true) ; enters at Close
)

(event EventBeginPlay)

(event Collision|EventActorBeginOverlap
  (params (OtherActor :type Actor%20Object%20Reference)))

(event EventTick
  (params (DeltaSeconds :type Float%20%28single-precision%29)))

(event Input|KeyboardEvents|F
  (params (Key :type Key%20Structure :default "None"))
  (:Pressed
    (Utilities|FlowControl|Gate true
      (:Exit
        (bind _outactors (Actor|GetAllActorsOfClass "/Game/Level/LEVEL1_CityStreet/Blueprints/Door_BP.Door_BP_C"))
        (Variables|/Game/Level/LEVEL1_CityStreet/Blueprints/Door_BP.Door_BP_C|SetDoorOpenActive (Utilities|Array|Get(acopy) _outactors) true)
        (Actor|DestroyActor)))))

(fn ConstructionScript)
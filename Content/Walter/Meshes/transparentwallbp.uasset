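; A transparent wall that acts as a progression gate, clearing only once every enemy grunt is gone.
; When the player character overlaps Bigbox, it searches the level for Enemy_Grunt actors and, if none remain, plays the Drop sequence and destroys itself after a short delay.
; The Smallbox hit event is empty, and leftover unconnected nodes hold unused "kill all enemies" message and Advance widget logic.
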(event OnComponentBeginOverlap(bigbox)
  (params (OverlappedComponent :type Primitive%20Component%20Object%20Reference) (OtherActor :type Actor%20Object%20Reference) (OtherComp :type Primitive%20Component%20Object%20Reference) (OtherBodyIndex :type Integer) (bFromSweep :type Boolean) (SweepResult :type Hit%20Result%20Structure%20%28by%20ref%29))
  (Utilities|Casting|CastToCube_PlayerCharacter OtherActor)
  (bind _outactors (Actor|GetAllActorsOfClass "/Game/Blueprints/Enemy/Enemy_Grunt.Enemy_Grunt_C"))
  (if (== (Utilities|Array|Length _outactors) 0)
    (Sequencer|Player|Play (Variables|/Script/ActorSequence.ActorSequenceComponent|GetSequencePlayer (Variables|Default|GetDrop)) :!class /Script/MovieScene.MovieSceneSequencePlayer)
    (Utilities|FlowControl|Delay 1.5)
    (Actor|DestroyActor)))

(event OnComponentHit(smallbox)
  (params (HitComponent :type Primitive%20Component%20Object%20Reference) (OtherActor :type Actor%20Object%20Reference) (OtherComp :type Primitive%20Component%20Object%20Reference) (NormalImpulse :type Vector :default "0, 0, 0") (Hit :type Hit%20Result%20Structure%20%28by%20ref%29)))

(fn ConstructionScript)
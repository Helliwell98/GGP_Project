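; Director actor that tracks Enemy_Grunts and manages horde spawning under a population cap.
; On BeginPlay it registers existing grunts and Hordespawners, binding to grunt kill events and spawner spawn requests.
; Requests spawn grunts at random reachable points near the given location, limited by Maxcreatures.
; Registering a grunt writes its array index to the player's EnemyCount; kills only remove it from the list.
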(event EventBeginPlay
  (Utilities|FlowControl|Sequence
    (:then_0
      (bind _outactors (Actor|GetAllActorsOfClass "/Game/Blueprints/Enemy/Enemy_Grunt.Enemy_Grunt_C"))
      (for _array_element _outactors
        (CallFunction|Oncreaturespawned _array_element)))
    (:then_1
      (bind _outactors_2 (Actor|GetAllActorsOfClass "/Game/Walter/spawn2/zombies/creature/director/gruntspawner/hordespawner.hordespawner_C"))
      (for _array_element_2 _outactors_2
        (CallFunction|Onhordespawnerspawned _array_element_2)))))

(event Collision|EventActorBeginOverlap
  (params (OtherActor :type Actor%20Object%20Reference)))

(fn ConstructionScript)

(fn Oncreaturespawned
  (params (enemygrunt :type Enemy%20Grunt%20Object%20Reference))
  (bind _returnvalue (Utilities|Array|Add (Variables|Default|GetEnemygrunts) enemygrunt))
  (bind _ascube_player_character (Utilities|Casting|CastToCube_PlayerCharacter (Game|Player|GetPlayerPawn 0)))
  (Variables|/Game/Blueprints/Player/Cube_PlayerCharacter.Cube_PlayerCharacter_C|SetEnemyCount _ascube_player_character _returnvalue)
  (EventDispatchers|BindEventtoOnkilled enemygrunt (EventDispatchers|CreateEvent :!event Oncreaturekilled)))

(fn Oncreaturekilled
  (params (enemygrunt :type Enemy%20Grunt%20Object%20Reference))
  (Utilities|Array|RemoveItem (Variables|Default|GetEnemygrunts) enemygrunt))

(fn Onhordespawnerspawned
  (params (hordespawners :type Hordespawner%20Object%20Reference))
  (Utilities|Array|Add (Variables|Default|Gethordespawnerrs) hordespawners)
  (EventDispatchers|BindEventtoRequestspawn hordespawners (EventDispatchers|CreateEvent :!event Oncreaturespawnedrequested)))

(fn Oncreaturespawnedrequested
  (params (count :type Integer) (location :type Vector))
  (for _index (range 1 (Math|Integer|Min(Integer) count (- (Variables|Default|Getmaxcreatures) (Utilities|Array|Length (Variables|Default|GetEnemygrunts)))))
    (bind _returnvalue (Game|SpawnActorfromClass "/Game/Blueprints/Enemy/Enemy_Grunt.Enemy_Grunt_C" (Math|Transform|MakeTransform (+ (.RandomLocation (AI|Navigation|GetRandomReachablePointinRadius location 2e+02 0 0)) "0, 0,100.000000") "0, 0, 0" "1,1,1") "AdjustIfPossibleButDontSpawnIfColliding" 0 0))
    (Utilities|IsValid _returnvalue
      (:Is%20Valid
        (CallFunction|Oncreaturespawned)))))
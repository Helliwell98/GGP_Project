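; Elite enemy character that chases the player and makes sequence-driven melee attacks, with randomized scale and yaw at spawn.
; AIMoveTo drives the chase; on arrival it plays the Attack sequence, waits a play-rate-scaled delay, damages a player overlapping DamBox, then re-chases.
; Taking damage halts the attack and briefly simulates capsule physics as a ragdoll stun, then resumes the chase and subtracts health, destroying the actor at zero.
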(event Custom|GruntDeath
  ;[1 1 1] Take Damage / Death
  (Actor|DestroyActor)
  (Development|PrintString "GruntDed"))

(event Custom|Chase%20Player
  (params (Player%20to%20chase :type Cube%20Player%20Character%20Object%20Reference))
  ;[1 1 1] AI Chase Player
  (if (not (Variables|Default|GetisRagdolling))
    (AI|AIMoveTo self "0, 0, 0" Player%20to%20chase 2e+02 false
      (:OnSuccess
        (Components|Movement|StopMovementImmediately (Variables|Character|GetCharacterMovement))
        (Sequencer|Player|Play (Variables|/Script/ActorSequence.ActorSequenceComponent|GetSequencePlayer (Variables|Default|GetAttack)) :!class /Script/MovieScene.MovieSceneSequencePlayer)
        (Utilities|FlowControl|Delay (/ 1.5 (Components|Animation|GetPlayRate (Variables|/Script/ActorSequence.ActorSequenceComponent|GetSequencePlayer (Variables|Default|GetAttack)))))
        (Development|PrintString "shoulddamage")
        (for _array_element (Collision|GetOverlappingActors (Variables|Default|GetDamBox) "/Game/Blueprints/Player/Cube_PlayerCharacter.Cube_PlayerCharacter_C" :!class /Script/Engine.PrimitiveComponent)
          _)
        (Utilities|FlowControl|DoOnce false :!label _label
          (:Completed
            (Game|Damage|ApplyDamage _array_element (Variables|Default|GetElite%20amage) 0 0)
            (Utilities|FlowControl|Delay 0.3)
            (Development|PrintString "ChacePlayer"))))
      (:OnFail
        _))
    (CallFunction|ChasePlayer (Variables|Default|GetCharacter%20Reference))
    (goto _label Reset)))

(event EventBeginPlay
  (bind _returnvalue (Math|Random|RandomFloatinRange 0.9 1.1))
  ;[1 1 1] AI Chase Player
  (Transformation|SetWorldScale3D (Variables|Character|GetMesh) (Math|Vector|MakeVector _returnvalue _returnvalue _returnvalue))
  (Transformation|SetActorRotation (Math|Rotator|MakeRotator 0.0 0.0 (Math|Random|RandomFloatinRange 0.0 3.6e+02)))
  (bind _ascube_player_character (Utilities|Casting|CastToCube_PlayerCharacter (Game|GetPlayerCharacter 0)))
  (bind _output_get (Variables|Default|SetCharacter%20Reference _ascube_player_character))
  (CallFunction|ChasePlayer _output_get))

(event Game|Damage|EventAnyDamage
  (params (Damage :type Float%20%28single-precision%29) (DamageType :type Damage%20Type%20Object%20Reference) (InstigatedBy :type Controller%20Object%20Reference) (DamageCauser :type Actor%20Object%20Reference))
  (bind _capsulecomponent (Variables|Collision|GetCapsuleComponent))
  ;[1 1 1] Take Damage / Death
  ;;[1 1 1] Ragdoll (Remove chase player)
  (Variables|Default|SetisRagdolling true)
  (Class|MovieSceneSequencePlayer|StopatCurrentTime (Variables|/Script/ActorSequence.ActorSequenceComponent|GetSequencePlayer (Variables|Default|GetAttack)))
  (Components|Movement|StopMovementImmediately (Variables|Character|GetCharacterMovement))
  (Physics|SetSimulatePhysics _capsulecomponent true)
  (Utilities|FlowControl|Delay 2.0)
  (Physics|SetSimulatePhysics _capsulecomponent false)
  (Variables|Default|SetisRagdolling false)
  (Transformation|SetWorldRotation (Variables|Collision|GetCapsuleComponent) "0, 0, 0" false false)
  (CallFunction|ChasePlayer (Variables|Default|GetCharacter%20Reference))
  (bind _output_get (Variables|Default|SetEliteHealth (Math|Float|Clamp(Float) (- (Variables|Default|GetEliteHealth) Damage) 0.0 5.0)))
  (Development|PrintString "GruntTakesDamage" true true "(R=0.000000,G=1.000000,B=0.070701,A=1.000000)")
  (if (== _output_get 0.0)
    (CallFunction|GruntDeath)))

(fn ConstructionScript)
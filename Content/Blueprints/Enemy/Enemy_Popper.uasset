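; Popper enemy that chases the player character and damages it on contact.
; On BeginPlay it caches the Cube player character and runs a looping AI MoveTo toward it.
; Each successful move waits briefly, applies damage and restarts the chase, while a failed move retries immediately.
; Incoming damage lowers its clamped health, and the actor destroys itself at zero.
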(event Custom|Chase%20Player
  (params (Player%20to%20chase :type Cube%20Player%20Character%20Object%20Reference))
  ;[1 1 1] AI Chase Player
  (AI|AIMoveTo self "0, 0, 0" Player%20to%20chase 5.0 false
    (:OnSuccess
      (Utilities|FlowControl|Delay 0.25)
      (Game|Damage|ApplyDamage (Game|GetPlayerCharacter 0) (Variables|Default|GetPopper%20Damage) 0 0)
      (Development|PrintString "Player Damaged" true true "(R=1.000000,G=0.956041,B=0.000000,A=1.000000)"))
    (:OnFail
      _))
  (CallFunction|ChasePlayer (Variables|Default|GetCharacter%20Reference)))

(event EventBeginPlay
  ;[1 1 1] AI Chase Player
  (bind _ascube_player_character (Utilities|Casting|CastToCube_PlayerCharacter (Game|GetPlayerCharacter 0)))
  (bind _output_get (Variables|Default|SetCharacter%20Reference _ascube_player_character))
  (CallFunction|ChasePlayer _output_get))

(event Game|Damage|EventAnyDamage
  (params (Damage :type Float%20%28single-precision%29) (DamageType :type Damage%20Type%20Object%20Reference) (InstigatedBy :type Controller%20Object%20Reference) (DamageCauser :type Actor%20Object%20Reference))
  ;[1 1 1] Take Damage / Death
  (bind _output_get (Variables|Default|SetPopperHealth (Math|Float|Clamp(Float) (- (Variables|Default|GetPopperHealth) Damage) 0.0 1.5e+02)))
  (if (== _output_get 0.0)
    (Actor|DestroyActor)))

(fn ConstructionScript)